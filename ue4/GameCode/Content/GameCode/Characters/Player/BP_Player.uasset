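; BP_Player is the player character Blueprint, adding a camera spring arm effect to sprinting.
; It stores the spring arm's default length on BeginPlay and extends the parent class's sprint start and stop events.
; A timeline lerps the arm between default and sprint lengths, playing forward on start and reversing on stop for a smooth transition.
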(event EventBeginPlay
  (Variables|SprintSettings|SetDefaultArmLength (Variables|/Script/Engine.SpringArmComponent|GetTargetArmLength (Variables|Default|GetSpringArmComponent))))

(event Collision|EventActorBeginOverlap
  (params (OtherActor :type Actor%20Object%20Reference)))

(event EventTick
  (params (DeltaSeconds :type Float%20%28single-precision%29)))

(event EventOnStartSprint
  (|CallParentFunction)
  (bind _newtrack_0 (Timeline|SpringLineTimeline Play)
    (:Update
      (Variables|/Script/Engine.SpringArmComponent|SetTargetArmLength (Variables|Default|GetSpringArmComponent) (Math|Float|Lerp (Variables|SprintSettings|GetDefaultArmLength) (Variables|SprintSettings|GetSprintArmLength) _newtrack_0)))))

(event EventOnStopSprint
  (|CallParentFunction)
  (bind _newtrack_0 (Timeline|SpringLineTimeline Reverse)
    (:Update
      (Variables|/Script/Engine.SpringArmComponent|SetTargetArmLength (Variables|Default|GetSpringArmComponent) (Math|Float|Lerp (Variables|SprintSettings|GetDefaultArmLength) (Variables|SprintSettings|GetSprintArmLength) _newtrack_0)))))

(fn ConstructionScript)